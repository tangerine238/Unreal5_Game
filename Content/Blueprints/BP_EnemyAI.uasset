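; Enemy AI Blueprint that chases the player on sight and performs a melee attack that knocks characters back.
; Pawn sensing triggers a move toward the player, and reaching them plays an attack montage, gated by a flag that resets when it completes or is interrupted.
; A montage notify runs a forward sphere trace that launches any hit Character forward and upward, with whoosh sounds on swing and hit.
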(event `self.PawnSensing.OnSeePawn`
  (params (Pawn :type "Pawn Object Reference"))
  (`self.Chase Player`))

(event `Chase Player`
  (bind _returnvalue (`self.K2_GetActorLocation`))
  (`|AIMoveTo` self (0.0 0.0 0.0) (`GameplayStatics.GetPlayerCharacter` 0) 120.0
    (:`OnSuccess`
      (if (`self.canAttack?`)
        (`|PlayMontage` (`self.Mesh`) "/Game/Characters/Villager/Animations/Attack/A_Attack_Montage.A_Attack_Montage"
          (:`then`
            (set `self.canAttack?` false)
            (`GameplayStatics.PlaySoundAtLocation` "/Game/Audio/MS_AxeWhoosh.MS_AxeWhoosh" (`self.K2_GetActorLocation`) (struct) 1.0 1.0 0.0 null null null null))
          (:`OnCompleted`
            (set `self.canAttack?` true :!label _label))
          (:`OnInterrupted`
            (goto _label))
          (:`OnNotifyBegin`
            (bind (_outhit _returnvalue_2) (`KismetSystemLibrary.SphereTraceSingle` _returnvalue (+ _returnvalue (* (`KismetMathLibrary.GetForwardVector` (`self.K2_GetActorRotation`)) 170.0)) 25.0 "TraceTypeQuery3"))
            (if _returnvalue_2
              (bind _ascharacter (cast `Character` (`.HitActor` (`GameplayStatics.BreakHitResult` _outhit))))
              (`self.LaunchCharacter` _ascharacter (+ (* (`KismetMathLibrary.GetForwardVector` (`self.K2_GetActorRotation`)) (`self.FrontalKnockback`)) (`KismetMathLibrary.MakeVector` 0.0 0.0 (`self.UpwardKnockback`))) false false)
              (`GameplayStatics.PlaySoundAtLocation` "/Game/Audio/MS_AxeWhoosh.MS_AxeWhoosh" (`self.K2_GetActorLocation`) (struct) 1.0 1.0 0.0 null null null null))))))))

(fn `UserConstructionScript`)